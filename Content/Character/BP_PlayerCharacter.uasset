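; Player character with movement, look, crouch and context actions for spraying graffiti and hammering statues.
; Tick picks the action from upward look or a short camera trace against actor tags and updates the HUD icon; Whistle and Fish have no behavior here.
; Painting locks movement, detaches the arm and drives a spawned decal through timelines while accruing FreedomPoints.
; Comparing camera and arm directions pauses painting when looking away.
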(event Custom|SetLookingStates
  (bind _returnvalue (Pawn|GetControlRotation :!class /Script/Engine.Pawn))
  ;[1 1 1] Set Looking States
  (Variables|Default|SetIsLookingDown (Math|Float|InRange(Float) (.pitch _returnvalue) 2.7e+02 3e+02))
  (Variables|Default|SetIsLookingUp (Math|Float|InRange(Float) (.pitch _returnvalue) 6e+01 9e+01))
  ;[1 1 1] Look Away From Graffiti
  (if (Variables|Default|GetIsGraffing)
    (if (< (Math|Vector|DotProduct (Math|Vector|GetForwardVector (Variables|Default|GetCamera)) (Math|Vector|GetForwardVector (Variables|Default|GetArm%20Holder))) 0.7)
      (CallFunction|PauseGraffiti)
      (else
        (CallFunction|ResumeGraffiti)))))

(event Custom|PauseGraffiti
  ;[1 1 1] Graffiti
  (Utilities|FlowControl|Sequence
    (:then_0
      (bind _newtrack_0 (Timeline|Timeline_2 Stop)
        (:Update
          (Default|ContinueGraffiti (Variables|Default|GetCurrent%20Graph) _newtrack_0))
        (:Finished
          (CallFunction|StopGraph))))
    (:then_1
      (Utilities|FlowControl|Gate true) ; enters at Close
    )
    (:then_2
      (Utilities|FlowControl|DoOnce false) ; enters at Reset
    )))

(event Custom|ResumeGraffiti
  ;[1 1 1] Graffiti
  (Utilities|FlowControl|Sequence
    (:then_0
      (Utilities|FlowControl|Gate true) ; enters at Open
    )
    (:then_1
      (Utilities|FlowControl|DoOnce false
        (:Completed
          (bind _newtrack_0 (Timeline|Timeline_2 Play)
            (:Update
              (Default|ContinueGraffiti (Variables|Default|GetCurrent%20Graph) _newtrack_0))
            (:Finished
              (CallFunction|StopGraph))))))))

(event Custom|StopGraph
  (bind _arm_holder (Variables|Default|GetArm%20Holder))
  ;[1 1 1] Graffiti
  (Class|SceneComponent|Attachto _arm_holder (Variables|Default|GetCamera) "None" "KeepRelativeOffset" true)
  (Transformation|ResetRelativeTransform _arm_holder)
  (Variables|Default|SetCurrent%20Graph 0)
  (Rendering|SetVisibility (Variables|Default|GetArmGraff) false false)
  (Variables|Default|SetIsGraffing false)
  (bind (_direction _newtrack_1 _newtrack_2) (Timeline|Timeline_1 Stop)
    (:Update
      (Transformation|SetRelativeRotation (Variables|Default|GetArmGraff) (Math|Rotator|MakeRotator 0.0 (* _newtrack_1 1e+01) (* _newtrack_2 1e+01)) false false)
      (Utilities|FlowControl|Gate true
        (:Exit
          (Variables|Default|SetFreedomPoints (+ (Variables|Default|GetFreedomPoints) (* 0.25 (Utilities|Time|GetWorldDeltaSeconds)))))))))

(event EventBeginPlay
  (bind _returnvalue (UserInterface|CreateWidget "/Game/Character/HUD/UI_HUD.UI_HUD_C" (Game|GetPlayerController 0)))
  (bind _output_get (Variables|Default|SetWidgetUI _returnvalue))
  (UserInterface|Viewport|AddtoViewport _output_get 0))

(event EventActorBeginOverlap
  (params (OtherActor :type Actor%20Object%20Reference)))

(event EventTick
  (params (DeltaSeconds :type Float%20%28single-precision%29))
  (bind _camera (Variables|Default|GetCamera))
  (bind _widgetui (Variables|Default|GetWidgetUI))
  (bind _returnvalue (Transformation|GetWorldLocation _camera))
  ;[1 1 1] Line Trace
  (if (not (Variables|Default|GetIsGraffing))
    (if (Variables|Default|GetIsLookingUp)
      (bind _output_get (Variables|Default|SetAvailableAction "NewEnumerator4"))
      (Default|SetIcon (Variables|Default|GetWidgetUI) _output_get)
      (else
        (bind (_outhit _returnvalue_2) (Collision|LineTraceForObjects _returnvalue (+ _returnvalue (* (Math|Vector|GetForwardVector _camera) 1.2e+02)) (Utilities|Array|MakeArray "ObjectTypeQuery5") false 0 "None"))
        (if _returnvalue_2
          (if (Actor|ActorHasTag (.HitActor (Collision|BreakHitResult _outhit)) "Graff")
            (bind _output_get_2 (Variables|Default|SetAvailableAction "NewEnumerator2"))
            (Default|SetIcon _widgetui _output_get_2)
            (elif (Actor|ActorHasTag (.HitActor (Collision|BreakHitResult _outhit)) "Guard")
              (bind _output_get_3 (Variables|Default|SetAvailableAction "NewEnumerator0"))
              (Default|SetIcon _widgetui _output_get_3)
              (elif (Actor|ActorHasTag (.HitActor (Collision|BreakHitResult _outhit)) "Statue")
                (bind _output_get_4 (Variables|Default|SetAvailableAction "NewEnumerator1"))
                (Default|SetIcon _widgetui _output_get_4)
                (else
                  ;[1 1 1] No Action In Range
                  (Default|HideIcon (Variables|Default|GetWidgetUI) :!label _label)
                  (Variables|Default|SetAvailableAction "NewEnumerator5")))))
          (else
            (goto _label)))))))

(event Input|ActionEvents|InputActionCrouch
  (params (Key :type Key%20Structure :default "AnyKey"))
  ;[1 1 1] Crouch
  (:Pressed
    (if (not (Variables|Default|GetIsGraffing))
      (Character|Crouch)))
  (:Released
    (Character|UnCrouch)))

(event Input|ActionEvents|InputActionAction
  (params (Key :type Key%20Structure :default "AnyKey"))
  (bind _armhammer (Variables|Default|GetArmHammer))
  (bind _arm_holder (Variables|Default|GetArm%20Holder))
  (bind _availableaction (Variables|Default|GetAvailableAction))
  (bind _armgraff (Variables|Default|GetArmGraff))
  (:Pressed
    (switch Utilities|FlowControl|Switch|SwitchonEnum_Actions _availableaction
      (:NewEnumerator1
        ;[1 1 1] Hammer
        (Rendering|SetVisibility (Variables|Default|GetArmHammer) true false)
        (bind _newtrack_0 (Timeline|Timeline_0 PlayFromStart)
          (:Update
            (Transformation|SetRelativeRotation _armhammer (Math|Rotator|MakeRotator -5.0 -11.0 _newtrack_0) false false))
          (:Finished
            (Rendering|SetVisibility _armhammer false false))))
      (:NewEnumerator2
        (if (Actor|ActorHasTag (.HitActor (Collision|BreakHitResult (stale EventTick _outhit))) "Graff")
          ;[1 1 1] Graffiti
          (Variables|/Script/Engine.Actor|SetTags (.HitActor (Collision|BreakHitResult (stale EventTick _outhit))) (Utilities|Array|MakeArray "None"))
          (Class|SceneComponent|DetachfromParent _arm_holder true true)
          (Rendering|SetVisibility _armgraff true false)
          (Variables|Default|SetIsGraffing true)
          (Utilities|FlowControl|Sequence
            (:then_0
              (bind _returnvalue (Game|SpawnActorfromClass "/Game/Character/Graffs/BP_DecalGraff.BP_DecalGraff_C" (Math|Transform|MakeTransform (.Location (Collision|BreakHitResult (stale EventTick _outhit))) (Math|Rotator|FindLookatRotation (.Location (Collision|BreakHitResult (stale EventTick _outhit))) (- (.Location (Collision|BreakHitResult (stale EventTick _outhit))) (.ImpactNormal (Collision|BreakHitResult (stale EventTick _outhit))))) "1,1,1") "Undefined" 0 0))
              (Variables|Default|SetCurrent%20Graph _returnvalue))
            (:then_1
              (bind _newtrack_0_2 (Timeline|Timeline_2 PlayFromStart)
                (:Update
                  (Default|ContinueGraffiti (Variables|Default|GetCurrent%20Graph) _newtrack_0_2))
                (:Finished
                  (CallFunction|StopGraph))))
            (:then_2
              (bind (_direction _newtrack_1 _newtrack_2) (Timeline|Timeline_1 PlayFromStart)
                (:Update
                  (Transformation|SetRelativeRotation (Variables|Default|GetArmGraff) (Math|Rotator|MakeRotator 0.0 (* _newtrack_1 1e+01) (* _newtrack_2 1e+01)) false false)
                  (Utilities|FlowControl|Gate true
                    (:Exit
                      (Variables|Default|SetFreedomPoints (+ (Variables|Default|GetFreedomPoints) (* 0.25 (Utilities|Time|GetWorldDeltaSeconds))))))))))
          (else
            (Development|PrintString "Has no tag!!" true true "(R=1.000000,G=0.000000,B=0.000000,A=1.000000)" 3.0))))))
  (:Released
    (switch Utilities|FlowControl|Switch|SwitchonEnum_Actions _availableaction
      (:NewEnumerator2
        (CallFunction|PauseGraffiti)
        (Class|SceneComponent|Attachto _arm_holder (Variables|Default|GetCamera) "None" "KeepRelativeOffset" true)
        (Transformation|ResetRelativeTransform _arm_holder)
        (Variables|Default|SetCurrent%20Graph 0)
        (Rendering|SetVisibility _armgraff false false)
        (Variables|Default|SetIsGraffing false)
        (Timeline|Timeline_1 Stop)))))

(event Input|AxisEvents|InputAxisMoveRight
  (params (AxisValue :type Float%20%28single-precision%29))
  ;[1 1 1] Move
  (if (not (Variables|Default|GetIsGraffing))
    (Pawn|Input|AddMovementInput (Transformation|GetActorRightVector) AxisValue false)))

(event Input|AxisEvents|InputAxisLookRight
  (params (AxisValue :type Float%20%28single-precision%29))
  ;[1 1 1] Look
  (Pawn|Input|AddControllerYawInput AxisValue)
  (CallFunction|SetLookingStates))

(event Input|AxisEvents|InputAxisLookUp
  (params (AxisValue :type Float%20%28single-precision%29))
  ;[1 1 1] Look
  (Pawn|Input|AddControllerPitchInput AxisValue)
  (CallFunction|SetLookingStates))

(event Input|AxisEvents|InputAxisMoveForward
  (params (AxisValue :type Float%20%28single-precision%29))
  ;[1 1 1] Move
  (if (not (Variables|Default|GetIsGraffing))
    (Pawn|Input|AddMovementInput (Transformation|GetActorForwardVector) AxisValue false)
    ;[1 1 1] Set Walking Back state
    (Variables|Default|SetIsWalkingBack (< AxisValue 0.0))))

(fn ConstructionScript)