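; Experimental guard vision-cone overlay, built as a fan of fixed triangle meshes spanning SightAngle out to ViewDistance.
; The construction script adds one rotated, scaled triangle per ray.
; While TraceRay is on, Tick line-traces each ray against WorldStatic and scales its triangle by hit time, so walls clip the cone without rebuilding geometry.
; ResetScale restores full reach, and ChangeMaterial picks the overlay material by GuardType.
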(event Custom|ResetScale
  (bind _viewdistance (Variables|Default|GetViewDistance))
  (bind _returnvalue (/ _viewdistance 3e+02))
  (for _array_element (Variables|Default|GetTriangleList)
    (Transformation|SetRelativeScale3D _array_element (Math|Vector|MakeVector (* _returnvalue (/ (/ (Variables|Default|GetSightAngle) (Math|Conversions|ToFloat(Integer) (Variables|Default|GetRayNb))) 6e+01)) _returnvalue 1.0))))

(event EventBeginPlay)

(event EventActorBeginOverlap
  (params (OtherActor :type Actor%20Object%20Reference)))

(event EventTick
  (params (DeltaSeconds :type Float%20%28single-precision%29))
  (bind _returnvalue (Transformation|GetActorLocation))
  (if (Variables|Default|GetTraceRay)
    (for _index (range 0 (- (Variables|Default|GetRayNb) 1))
      (bind _outhit (Collision|LineTraceForObjects _returnvalue (+ _returnvalue (Math|Vector|RotateVectorAroundAxis (* (Transformation|GetActorRightVector) (Variables|Default|GetViewDistance)) (+ (* _index (/ (Variables|Default|GetSightAngle) (Math|Conversions|ToFloat(Integer) (Variables|Default|GetRayNb)))) (/ (- 1.8e+02 (Variables|Default|GetSightAngle)) 2.0) (/ (/ (Variables|Default|GetSightAngle) (Math|Conversions|ToFloat(Integer) (Variables|Default|GetRayNb))) 2.0)) "0, 0,1.000000")) (Utilities|Array|MakeArray "ObjectTypeQuery1") false 0 "None"))
      (Transformation|SetRelativeScale3D (Utilities|Array|Get(acopy) (Variables|Default|GetTriangleList) _index) (Math|Vector|MakeVector (* (* (.Time (Collision|BreakHitResult _outhit)) (/ (Variables|Default|GetViewDistance) 3e+02)) (/ (/ (Variables|Default|GetSightAngle) (Math|Conversions|ToFloat(Integer) (Variables|Default|GetRayNb))) 6e+01)) (* (.Time (Collision|BreakHitResult _outhit)) (/ (Variables|Default|GetViewDistance) 3e+02)) 1.0)))))

(fn ConstructionScript
  (for _index (range 0 (- (Variables|Default|GetRayNb) 1))
    (bind _returnvalue (AddComponent|AddStaticMeshComponent false (Math|Transform|MakeTransform "0, 0, 0" (Math|Rotator|MakeRotator 0.0 0.0 (+ (* _index (/ (Variables|Default|GetSightAngle) (Math|Conversions|ToFloat(Integer) (Variables|Default|GetRayNb)))) (/ (- 1.8e+02 (Variables|Default|GetSightAngle)) 2.0) (/ (/ (Variables|Default|GetSightAngle) (Math|Conversions|ToFloat(Integer) (Variables|Default|GetRayNb))) 2.0) 1.8e+02)) (Math|Vector|MakeVector (* (/ (Variables|Default|GetViewDistance) 3e+02) (/ (/ (Variables|Default|GetSightAngle) (Math|Conversions|ToFloat(Integer) (Variables|Default|GetRayNb))) 6e+01)) (/ (Variables|Default|GetViewDistance) 3e+02) 1.0))))
    (Utilities|Array|Add (Variables|Default|GetTriangleList) _returnvalue)))

(fn ChangeMaterial
  (for _array_element (Variables|Default|GetTriangleList)
    (Rendering|Material|SetMaterial _array_element 0 (Utilities|Select :Index (Variables|Default|GetGuardType) :NewEnumerator0 "/Game/Experimental/M_GuardOverlay_3.M_GuardOverlay_3" :NewEnumerator1 "/Game/Experimental/M_GuardOverlay_2.M_GuardOverlay_2" :NewEnumerator2 "/Game/Experimental/M_GuardOverlay.M_GuardOverlay"))))