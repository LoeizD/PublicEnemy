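; BP_Statue is a breakable statue that alerts guards when destroyed.
; Its Break event disables box collision, shatters the destructible mesh away from the player's facing direction, plays a break sound and sets a five-second lifespan.
; It then calls StatueIsBroken on every BP_Guard in the level and spawns a new guard through the player's current tile.
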(event Custom|Break
  (bind _breakstat (Variables|Default|GetBreakStat))
  (Collision|SetCollisionEnabled (Variables|Default|GetBox) "NoCollision")
  (Game|Damage|ApplyDamage (Variables|Default|GetSM_Statue_DM) 5e+02 (Transformation|GetWorldLocation (Variables|Default|GetDefaultSceneRoot)) (Transformation|GetActorForwardVector (Game|Player|GetPlayerPawn 0)) 2e+03)
  (Actor|SetLifeSpan 5.0)
  (Class|FMODAudioComponent|Play _breakstat)
  (Class|FMODAudioComponent|SetVolume _breakstat 0.5)
  (Utilities|FlowControl|Sequence
    (:then_0
      (bind _outactors (Actor|GetAllActorsOfClass "/Game/Blueprints/Guard/BP_Guard.BP_Guard_C"))
      (for _array_element _outactors
        (Default|StatueIsBroken _array_element)))
    (:then_1
      (Default|SpawnGuard (Variables|/Game/Character/BP_PlayerCharacter.BP_PlayerCharacter_C|GetCurrentTile (.AsBP%20Player%20Character (Utilities|Casting|CastToBP_PlayerCharacter (Game|Player|GetPlayerPawn 0)))) "0, 0, 0"))))

(fn ConstructionScript)