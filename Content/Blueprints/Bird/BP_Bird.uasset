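; BP_Bird is a bird actor that animates a morph target and flies in a straight line once triggered.
; After a random startup delay, which varies timing between instances, a timeline drives the "fly" morph target on the SMBird mesh.
; The Fly event shows the mesh and enables movement, so Tick then moves it along relative X at constant, frame-rate-independent speed.
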(event Custom|Fly
  (Variables|Default|SetCanFly true)
  (Rendering|SetVisibility (Variables|Default|GetSM_Bird) true false))

(event EventBeginPlay
  (Utilities|FlowControl|Delay (Math|Random|RandomFloatinRange 0.0 0.8))
  (bind _newtrack_3 (Timeline|Timeline_0 Play)
    (:Update
      (Components|SkeletalMesh|SetMorphTarget (Variables|Default|GetSM_Bird) "fly" _newtrack_3 true))))

(event EventTick
  (params (DeltaSeconds :type Float%20%28single-precision%29))
  (if (Variables|Default|GetCanFly)
    (Transformation|AddRelativeLocation (Variables|Default|GetSM_Bird) (Math|Vector|MakeVector (* DeltaSeconds 3e+02) 0.0 0.0) false false)))

(fn ConstructionScript)