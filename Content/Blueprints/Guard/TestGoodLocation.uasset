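; Test Blueprint in the Guard folder that scatters the arrow components under Scene to random navigable locations on BeginPlay.
; For each arrow, it samples reachable points using half the diagonal between two corner variables as radius, retrying until the X/Y bounds test passes.
; The random query is re-evaluated when setting the target, so the placed point, flattened to Z=0, can differ from the tested one.
; An IsValidAILocation check that stretches the arrow is disconnected.
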(event EventBeginPlay
  (bind _navigationlocation_corner_hautdroite (Variables|Default|GetNavigationLocation_Corner_HautDroite))
  (bind _navigationlocation_corner_basgauche (Variables|Default|GetNavigationLocation_Corner_BasGauche))
  (bind _navigationlocation_corner_hautdroite_2 (Variables|Default|GetNavigationLocation_Corner_HautDroite))
  (bind _navigationlocation_corner_basgauche_2 (Variables|Default|GetNavigationLocation_Corner_BasGauche))
  (bind _returnvalue (- _navigationlocation_corner_hautdroite_2 _navigationlocation_corner_basgauche_2))
  (bind _returnvalue_2 (Math|Vector|VectorLength _returnvalue))
  (bind _returnvalue_3 (/ _returnvalue_2 2.0))
  (bind _returnvalue_4 (AI|Navigation|GetRandomReachablePointinRadius (Math|Vector|MakeVector 0.0 0.0 0.0) _returnvalue_3 0 "/Script/Engine.NavigationQueryFilter"))
  (bind _returnvalue_5 (Math|Vector|MakeVector (.x _returnvalue_4) (.y _returnvalue_4) 0.0))
  (for _array_element (Components|GetChildrenComponents (Variables|Default|GetScene) false)
    (bind _asarrow_component (Utilities|Casting|CastToArrowComponent _array_element))
    (if (Math|Boolean|ANDBoolean (> (.x _returnvalue_4) (.x _navigationlocation_corner_basgauche)) (< (.x _returnvalue_4) (.x _navigationlocation_corner_hautdroite)) (> (.y _returnvalue_4) (.y _navigationlocation_corner_hautdroite)) (< (.y _returnvalue_4) (.y _navigationlocation_corner_basgauche))) :!label _label
      (bind _output_get (Variables|Default|SetChosenTarget _returnvalue_5))
      (Transformation|SetWorldLocation _asarrow_component _output_get false false)
      (else
        (Variables|Default|SetChosenTarget _returnvalue_5)
        (goto _label)))))

(fn ConstructionScript)