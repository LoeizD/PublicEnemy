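; Guard character that wanders a rectangular navigation area and stops to face the player when they enter its suspicion box.
; A Tick-driven state machine runs timed look-around (curve-based yaw), turn-over and shocked jump states, plus go-to moves with a stuck timeout.
; Weighted random Selects pick the next state, with a flag limiting repeated turn-overs.
; Go-to targets come from retried random navmesh queries, and construction randomises a guard style label.
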(event OnComponentBeginOverlap(Box)
  (params (OtherActor :type Actor%20Object%20Reference) (OtherComp :type Primitive%20Component%20Object%20Reference) (OtherBodyIndex :type Integer) (bFromSweep :type Boolean) (SweepResult :type Hit%20Result%20Structure%20%28by%20ref%29))
  (Utilities|Casting|CastToBP_PlayerCharacter OtherActor)
  (Development|PrintString "SALO !!!!!!!!!")
  (Variables|Default|SetPlayerIsInHisSuspiciousZone true)
  (Components|Movement|StopMovementImmediately (Variables|Character|GetCharacterMovement))
  (Variables|Default|SetGuard_State "NewEnumerator4"))

(event OnComponentEndOverlap(Box)
  (params (OtherActor :type Actor%20Object%20Reference) (OtherComp :type Primitive%20Component%20Object%20Reference) (OtherBodyIndex :type Integer))
  (Utilities|Casting|CastToBP_PlayerCharacter OtherActor)
  (Variables|Default|SetPlayerIsInHisSuspiciousZone false)
  (CallFunction|ChooseAnotherState))

(event EventBeginPlay
  (bind _outactors (Actor|GetAllActorsOfClass "/Script/Engine.TargetPoint"))
  (Variables|Default|SetWaypoints _outactors))

(event EventTick
  (params (DeltaSeconds :type Float%20%28single-precision%29))
  (bind _returnvalue (Transformation|GetActorLocation))
  (bind _rotationwhenbeginstate (Variables|Default|GetRotationWhenBeginState))
  (bind _rotationwhenbeginstate_2 (Variables|Default|GetRotationWhenBeginState))
  (bind _chosentarget (Variables|Default|GetChosenTarget))
  (CallFunction|CheckifStateChanged)
  (switch Utilities|FlowControl|Switch|SwitchonGuard_States (Variables|Default|GetGuard_State)
    (:NewEnumerator0
      (if (Variables|Default|GetStateWasDifferentAtPreviousFrame)
        (CallFunction|InitStateTimer)
        (CallFunction|SaveActorRotation))
      (Utilities|UpdateTimer
        (:NotFinished
          (bind _output_get (Variables|Default|SetState_Percentage (/ (Math|Float|%(Float) (Variables|Default|GetState_ActualTimer) (Variables|LookAround|GetState_LookAround_Period)) (Variables|LookAround|GetState_LookAround_Period)))) ; Override le percentage\ncalculé par UpdateTimer
          (Transformation|SetWorldRotation (Variables|Collision|GetCapsuleComponent) (Math|Rotator|MakeRotator (.roll _rotationwhenbeginstate) (.pitch _rotationwhenbeginstate) (+ (.yaw _rotationwhenbeginstate) (* (Math|Curves|GetFloatValue (Variables|LookAround|GetCRV_LookAround) _output_get) (Variables|LookAround|GetState_LookAround_Angle)))) false false))
        (:Finished
          (CallFunction|ChooseAnotherState))))
    (:NewEnumerator1
      (if (Variables|Default|GetStateWasDifferentAtPreviousFrame)
        (CallFunction|InitStateTimer)
        (CallFunction|SaveActorRotation)
        (Variables|Default|SetSecuAntiMultiTurnOver true)
        (Variables|TurnOver|SetState_TurnOver_Side (select (Math|Random|RandomBool) -1.0 1.0)))
      (Utilities|UpdateTimer
        (:NotFinished
          (Transformation|SetWorldRotation (Variables|Collision|GetCapsuleComponent) (Math|Rotator|MakeRotator (.roll _rotationwhenbeginstate_2) (.pitch _rotationwhenbeginstate_2) (+ (.yaw _rotationwhenbeginstate_2) (* (Variables|Default|GetState_Percentage) (Variables|TurnOver|GetState_TurnOver_Side) 1.8e+02))) false false))
        (:Finished
          (CallFunction|ChooseAnotherState))))
    (:NewEnumerator3
      (if (Variables|Default|GetStateWasDifferentAtPreviousFrame)
        (CallFunction|MovetoANewPoint)
        (Variables|Default|SetState_GoTo_SecureActualTimer 0.0)
        (else
          ;[1 1 1] Test si arrivé à destination
          (if (< (Math|Vector|VectorLength (- (Math|Vector|MakeVector (.x _chosentarget) (.y _chosentarget) 0.0) (Math|Vector|MakeVector (.x _returnvalue) (.y _returnvalue) 0.0))) 2.0)
            (CallFunction|ChooseAnotherState)
            (else
              ;[1 1 1] Si le garde reste kéblo trop longtemps, il cherche un autre objectif
              (if (< (Math|Vector|VectorLength (Variables|/Script/Engine.MovementComponent|GetVelocity (Variables|Character|GetCharacterMovement))) 0.2) ; Si le garde est bloqué
                (bind _output_get_2 (Variables|Default|SetState_GoTo_SecureActualTimer (+ (Variables|Default|GetState_GoTo_SecureActualTimer) (Utilities|Time|GetWorldDeltaSeconds)))) ; Sinon, on reset le timer de sécu
                (if (> _output_get_2 (Variables|Default|GetState_GoTo_SecureTimerDuration))
                  (Development|PrintString "OH MY GOD J'ETAIS COMPLETEMENT BLOQUE !!!!!! Donc je vais à un autre endroit... " true true "(R=0.000000,G=0.660000,B=1.000000,A=1.000000)" 1e+02)
                  (CallFunction|MovetoANewPoint)
                  (Variables|Default|SetState_GoTo_SecureActualTimer 0.0))
                (else
                  (Variables|Default|SetState_GoTo_SecureActualTimer 0.0) ; Sinon, on reset le timer de sécu
                )))))))
    (:NewEnumerator4
      (Transformation|SetActorRotation (Math|Rotator|FindLookatRotation (Transformation|GetActorLocation) (Transformation|GetActorLocation (.AsBP%20Player%20Character (Utilities|Casting|CastToBP_PlayerCharacter (Game|Player|GetPlayerPawn 0)))))))
    (:NewEnumerator5)
    (:NewEnumerator6
      (if (Variables|Default|GetStateWasDifferentAtPreviousFrame)
        (CallFunction|InitStateTimer)
        (Character|Jump))
      (Utilities|UpdateTimer
        (:Finished
          (CallFunction|ChooseAnotherState))))))

(fn ConstructionScript
  (bind _output_get (Variables|Default|SetGuard_Style (Utilities|Select :Index (Math|Random|RandomIntegerinRange 0 2) :Option%200 "NewEnumerator0" :Option%201 "NewEnumerator1" :Option%202 "NewEnumerator2")))
  (Rendering|Components|TextRender|SetText (Variables|Default|GetStyle) (Utilities|Select :Index _output_get :NewEnumerator0 (LocalVariables|GetDown) :NewEnumerator1 (LocalVariables|GetCrouch) :NewEnumerator2 (LocalVariables|GetBack))))

(fn CheckifStateChanged
  (if (Utilities|Enum|NotEqual(Enum) (Variables|Default|GetGuard_State) (Variables|Default|GetGuad_StateAtPreviousFrame))
    (Variables|Default|SetStateWasDifferentAtPreviousFrame true)
    (Variables|Default|SetGuad_StateAtPreviousFrame (Variables|Default|GetGuard_State))
    (else
      (Variables|Default|SetStateWasDifferentAtPreviousFrame false)))
  (return))

(fn InitStateTimer
  (Variables|Default|SetState_TimerDuration (Utilities|Select :Index (Variables|Default|GetGuard_State) :NewEnumerator2 0.0 :NewEnumerator0 (Math|Random|RandomFloatinRange (Variables|LookAround|GetState_LookAround_MinDuration) (Variables|LookAround|GetState_LookAround_MaxDuration)) :NewEnumerator1 (Math|Random|RandomFloatinRange (Variables|TurnOver|GetState_TurnOver_MinDuration) (Variables|TurnOver|GetState_TurnOver_MaxDuration)) :NewEnumerator3 0.0 :NewEnumerator4 0.0 :NewEnumerator5 0.0 :NewEnumerator6 (Variables|State_Shocked|GetState_Shocked_TimerDuration)))
  (Variables|Default|SetState_ActualTimer 0.0))

(fn ChooseAnotherState
  ;[1 1 1] Sécu anti double TurnOver
  (if (and (Utilities|Enum|NotEqual(Enum) (Variables|Default|GetGuard_State) "NewEnumerator1") (Utilities|Enum|NotEqual(Enum) (Variables|Default|GetGuard_State) "NewEnumerator0"))
    (Variables|Default|SetSecuAntiMultiTurnOver false))
  (Variables|Default|SetGuard_State (Utilities|Select :Index (Variables|Default|GetGuard_State) :NewEnumerator2 "NewEnumerator3" :NewEnumerator0 (select (Variables|Default|GetSecuAntiMultiTurnOver) "NewEnumerator3" (Utilities|Select :Index (Math|Random|RandomIntegerinRange 0 3) :Option%200 "NewEnumerator1" :Option%201 "NewEnumerator3" :Option%202 "NewEnumerator3" :Option%203 "NewEnumerator3")) :NewEnumerator1 "NewEnumerator0" :NewEnumerator3 (Utilities|Select :Index (Math|Random|RandomIntegerinRange 0 4) :Option%200 "NewEnumerator1" :Option%201 "NewEnumerator0" :Option%202 "NewEnumerator3" :Option%203 "NewEnumerator3" :Option%204 "NewEnumerator3") :NewEnumerator4 "NewEnumerator3" :NewEnumerator5 "NewEnumerator6" :NewEnumerator6 (Utilities|Select :Index (Math|Random|RandomIntegerinRange 0 2) :Option%200 "NewEnumerator1" :Option%201 "NewEnumerator3" :Option%202 "NewEnumerator3"))))

(fn SaveActorRotation
  (Variables|Default|SetRotationWhenBeginState (Transformation|GetWorldRotation (Variables|Collision|GetCapsuleComponent)))
  (return))

(fn MovetoANewPoint
  (bind _navigationlocation_corner_hautdroite (Variables|Default|GetNavigationLocation_Corner_HautDroite))
  (bind _navigationlocation_corner_basgauche (Variables|Default|GetNavigationLocation_Corner_BasGauche))
  (bind _navigationlocation_corner_hautdroite_2 (Variables|Default|GetNavigationLocation_Corner_HautDroite))
  (bind _navigationlocation_corner_basgauche_2 (Variables|Default|GetNavigationLocation_Corner_BasGauche))
  (bind _returnvalue (- _navigationlocation_corner_hautdroite_2 _navigationlocation_corner_basgauche_2))
  (bind _returnvalue_2 (Math|Vector|VectorLength _returnvalue))
  (bind _returnvalue_3 (/ _returnvalue 2.0))
  (bind _returnvalue_4 (/ _returnvalue_2 2.0))
  (bind _returnvalue_5 (+ _returnvalue_3 _navigationlocation_corner_basgauche_2))
  (bind _returnvalue_6 (AI|Navigation|GetRandomReachablePointinRadius (Math|Vector|MakeVector (.x _returnvalue_5) (.y _returnvalue_5) 0.0) _returnvalue_4 0 "/Script/Engine.NavigationQueryFilter"))
  (bind _returnvalue_7 (Math|Vector|MakeVector (.x _returnvalue_6) (.y _returnvalue_6) 0.0))
  (if (Math|Boolean|ANDBoolean (> (.x _returnvalue_6) (.x _navigationlocation_corner_basgauche)) (< (.x _returnvalue_6) (.x _navigationlocation_corner_hautdroite)) (> (.y _returnvalue_6) (.y _navigationlocation_corner_hautdroite)) (< (.y _returnvalue_6) (.y _navigationlocation_corner_basgauche))) :!label _label
    (bind _output_get (Variables|Default|SetChosenTarget _returnvalue_7))
    (AI|Navigation|SimpleMovetoLocation (Pawn|GetController) _output_get)
    (else
      (Variables|Default|SetChosenTarget _returnvalue_7)
      (goto _label))))