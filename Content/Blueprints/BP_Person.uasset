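; Wandering crowd character that walks between random navigable points in a zone set by two corners, with a random color applied at construction.
; Tick picks a new target when none is set, movement stalls or arrival occurs, sometimes after a short random rest.
; GoToPointInZone retries random points until one passes the bounds check, but re-rolls the stored target, then randomizes ArchVis walk speed and calls SimpleMoveToLocation.
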(event Custom|LittleRest
  (Utilities|FlowControl|Delay (Math|Random|RandomFloatinRange 0.5 2.0))
  (CallFunction|GotoPointinZone)
  (Variables|Default|SetTakeARest false))

(event EventBeginPlay)

(event EventTick
  (params (DeltaSeconds :type Float%20%28single-precision%29))
  (bind _returnvalue (Transformation|GetActorLocation))
  (bind _chosentarget (Variables|Default|GetChosenTarget))
  (if (not (Variables|Default|GetTakeARest))
    ;[1 1 1] Utile seulement au début
    (if (Math|Vector|Equal(Vector) (Variables|Default|GetChosenTarget) "0, 0, 0" 0.0001)
      (CallFunction|GotoPointinZone)
      (else
        ;[1 1 1] SECU pour quand ils restent bloqués dans leur déplacement...
        (if (< (Math|Vector|VectorLength (Variables|/Script/Engine.MovementComponent|GetVelocity (Variables|Character|GetCharacterMovement))) 0.1)
          (CallFunction|GotoPointinZone)
          (else
            ;[1 1 1] Test si arrivé à destination
            (if (< (Math|Vector|VectorLength (- (Math|Vector|MakeVector (.x _chosentarget) (.y _chosentarget) 0.0) (Math|Vector|MakeVector (.x _returnvalue) (.y _returnvalue) 0.0))) 1e+02)
              ;[1 1 1] Prennent une petit pause, choix rando
              (if (Math|Random|RandomBool)
                (Variables|Default|SetTakeARest true)
                (CallFunction|LittleRest)
                (else
                  (CallFunction|GotoPointinZone))))))))))

(fn ConstructionScript
  (bind _returnvalue (Rendering|Material|CreateDynamicMaterialInstance (Variables|Default|GetPerson) 0 0 :!class /Script/Engine.PrimitiveComponent))
  (Rendering|Material|SetVectorParameterValue _returnvalue "Color" (Utilities|Struct|MakeLinearColor (Math|Random|RandomFloatinRange 0.0 1.0) (Math|Random|RandomFloatinRange 0.0 1.0) (Math|Random|RandomFloatinRange 0.0 1.0) 0.0) :!class /Script/Engine.MaterialInstanceDynamic))

(fn GotoPointinZone
  (bind _navigationlocation_corner_hautdroite (Variables|Default|GetNavigationLocation_Corner_HautDroite))
  (bind _navigationlocation_corner_basgauche (Variables|Default|GetNavigationLocation_Corner_BasGauche))
  (bind _navigationlocation_corner_hautdroite_2 (Variables|Default|GetNavigationLocation_Corner_HautDroite))
  (bind _navigationlocation_corner_basgauche_2 (Variables|Default|GetNavigationLocation_Corner_BasGauche))
  (bind _returnvalue (- _navigationlocation_corner_hautdroite_2 _navigationlocation_corner_basgauche_2))
  (bind _returnvalue_2 (Math|Vector|VectorLength _returnvalue))
  (bind _returnvalue_3 (/ _returnvalue 2.0))
  (bind _returnvalue_4 (/ _returnvalue_2 2.0))
  (bind _returnvalue_5 (+ _returnvalue_3 _navigationlocation_corner_basgauche_2))
  (bind _returnvalue_6 (AI|Navigation|GetRandomReachablePointinRadius (Math|Vector|MakeVector (.x _returnvalue_5) (.y _returnvalue_5) 0.0) _returnvalue_4 0 "/Script/Engine.NavigationQueryFilter"))
  (bind _returnvalue_7 (Math|Vector|MakeVector (.x _returnvalue_6) (.y _returnvalue_6) 0.0))
  (if (Math|Boolean|ANDBoolean (> (.x _returnvalue_6) (.x _navigationlocation_corner_basgauche)) (< (.x _returnvalue_6) (.x _navigationlocation_corner_hautdroite)) (> (.y _returnvalue_6) (.y _navigationlocation_corner_hautdroite)) (< (.y _returnvalue_6) (.y _navigationlocation_corner_basgauche))) :!label _label
    (bind _output_get (Variables|Default|SetChosenTarget _returnvalue_7))
    (Utilities|FlowControl|Sequence
      (:then_0
        (bind _asarch_vis_char_movement_component (Utilities|Casting|CastToArchVisCharMovementComponent (Variables|Character|GetCharacterMovement)))
        (Variables|/Script/Engine.CharacterMovementComponent|SetMaxWalkSpeed _asarch_vis_char_movement_component (Math|Random|RandomFloatinRange (Variables|Default|GetMinSpeed) (Variables|Default|GetMaxSpeed))))
      (:then_1
        (AI|Navigation|SimpleMovetoLocation (Pawn|GetController) _output_get)
        (return)))
    (else
      (Variables|Default|SetChosenTarget _returnvalue_7)
      (goto _label))))