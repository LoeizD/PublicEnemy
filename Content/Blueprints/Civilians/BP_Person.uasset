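; Civilian character that wanders inside a rectangular zone, with a random tint and footstep sound picked at construction.
; GoToPointInZone retries random reachable navmesh points until one passes the corner bounds check, then sends a simple move at random walk speed.
; Tick re-picks targets when movement stalls, randomly pauses or moves on at arrival, and plays footsteps at an interval scaled to speed.
; Older TargetPoint waypoint logic remains unconnected.
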(event Custom|LittleRest
  (Utilities|FlowControl|Delay (Math|Random|RandomFloatinRange 0.5 2.0))
  (CallFunction|GotoPointinZone)
  (Variables|Default|SetTakeARest false))

(event EventBeginPlay)

(event EventTick
  (params (DeltaSeconds :type Float%20%28single-precision%29))
  (bind _returnvalue (Transformation|GetActorLocation))
  (bind _walk_timerduration (Variables|Default|GetWalk_TimerDuration))
  (bind _chosentarget (Variables|Default|GetChosenTarget))
  (if (not (Variables|Default|GetTakeARest))
    ;[1 1 1] Utile seulement au début
    (if (Math|Vector|Equal(Vector) (Variables|Default|GetChosenTarget) "0, 0, 0" 0.0001)
      (CallFunction|GotoPointinZone)
      (else
        ;[1 1 1] SECU pour quand ils restent bloqués dans leur déplacement...
        (if (< (Math|Vector|VectorLength (Variables|/Script/Engine.MovementComponent|GetVelocity (Variables|Character|GetCharacterMovement))) 0.1)
          (CallFunction|GotoPointinZone)
          (else
            ;[1 1 1] Test si arrivé à destination
            (if (< (Math|Vector|VectorLength (- (Math|Vector|MakeVector (.x _chosentarget) (.y _chosentarget) 0.0) (Math|Vector|MakeVector (.x _returnvalue) (.y _returnvalue) 0.0))) 1e+02)
              ;[1 1 1] Prennent une petit pause, choix rando
              (if (Math|Random|RandomBool)
                (Variables|Default|SetTakeARest true)
                (CallFunction|LittleRest)
                (else
                  (CallFunction|GotoPointinZone)))
              (else
                ;[1 1 1] Bruits de pas
                (bind _output_get (Variables|Default|SetWalk_ActualTimer (+ (Variables|Default|GetWalk_ActualTimer) (Utilities|Time|GetWorldDeltaSeconds))))
                (if (>= _output_get _walk_timerduration)
                  (CallFunction|PlaySFXWalk)
                  (Variables|Default|SetWalk_ActualTimer (Math|Float|%(Float) _output_get _walk_timerduration)))))))))))

(fn ConstructionScript
  (bind _returnvalue (Rendering|Material|CreateDynamicMaterialInstance (Variables|Default|GetPerson) 0 0 :!class /Script/Engine.PrimitiveComponent))
  (Rendering|Material|SetVectorParameterValue _returnvalue "Color" (Utilities|Struct|MakeLinearColor (Math|Random|RandomFloatinRange 0.0 1.0) (Math|Random|RandomFloatinRange 0.0 1.0) (Math|Random|RandomFloatinRange 0.0 1.0) 0.0) :!class /Script/Engine.MaterialInstanceDynamic)
  (Variables|Default|SetMyWalkSFX (Utilities|Select :Index (Math|Random|RandomIntegerinRange 0 3) :Option%200 (Variables|Default|GetWalk_1) :Option%201 (Variables|Default|GetWalk_2) :Option%202 (Variables|Default|GetWalk_3) :Option%203 (Variables|Default|GetWalk_4))))

(fn GotoPointinZone
  (bind _navigationlocation_corner_hautdroite (Variables|Default|GetNavigationLocation_Corner_HautDroite))
  (bind _navigationlocation_corner_basgauche (Variables|Default|GetNavigationLocation_Corner_BasGauche))
  (bind _navigationlocation_corner_hautdroite_2 (Variables|Default|GetNavigationLocation_Corner_HautDroite))
  (bind _navigationlocation_corner_basgauche_2 (Variables|Default|GetNavigationLocation_Corner_BasGauche))
  (bind _returnvalue (- _navigationlocation_corner_hautdroite_2 _navigationlocation_corner_basgauche_2))
  (bind _returnvalue_2 (Math|Vector|VectorLength _returnvalue))
  (bind _returnvalue_3 (/ _returnvalue 2.0))
  (bind _returnvalue_4 (/ _returnvalue_2 2.0))
  (bind _returnvalue_5 (+ _returnvalue_3 _navigationlocation_corner_basgauche_2))
  (bind _returnvalue_6 (AI|Navigation|GetRandomReachablePointinRadius (Math|Vector|MakeVector (.x _returnvalue_5) (.y _returnvalue_5) 0.0) _returnvalue_4 0 "/Script/Engine.NavigationQueryFilter"))
  (bind _returnvalue_7 (Math|Vector|MakeVector (.x _returnvalue_6) (.y _returnvalue_6) 0.0))
  (if (Math|Boolean|ANDBoolean (> (.x _returnvalue_6) (.x _navigationlocation_corner_basgauche)) (< (.x _returnvalue_6) (.x _navigationlocation_corner_hautdroite)) (> (.y _returnvalue_6) (.y _navigationlocation_corner_hautdroite)) (< (.y _returnvalue_6) (.y _navigationlocation_corner_basgauche))) :!label _label
    (bind _output_get (Variables|Default|SetChosenTarget _returnvalue_7))
    (Utilities|FlowControl|Sequence
      (:then_0
        ;[1 1 1] Vitesse de pas
        (bind _output_get_2 (Variables|/Script/Engine.CharacterMovementComponent|SetMaxWalkSpeed (Variables|Character|GetCharacterMovement) (Math|Random|RandomFloatinRange (Variables|Default|GetMinSpeed) (Variables|Default|GetMaxSpeed))))
        ;[1 1 1] Calcul de la fréquence de sin de pas en fonction de la vitesse
        (bind _output_get_3 (Variables|Default|SetWalk_TimerDuration (- (Variables|Default|GetSFX_Walk_LowSpeed) (* (/ (- _output_get_2 (Variables|Default|GetMinSpeed)) (- (Variables|Default|GetMaxSpeed) (Variables|Default|GetMinSpeed))) (- (Variables|Default|GetSFX_Walk_LowSpeed) (Variables|Default|GetSFX_Walk_HighSpeed))))))
        (Development|PrintString (Utilities|String|ToString(Float) _output_get_3) true true "(R=0.000000,G=0.660000,B=1.000000,A=1.000000)" 1e+02))
      (:then_1
        (AI|Navigation|SimpleMovetoLocation (Pawn|GetController) _output_get)
        (return)))
    (else
      (Variables|Default|SetChosenTarget _returnvalue_7)
      (goto _label))))

(fn PlaySFXWalk
  (Class|FMODAudioComponent|Play (Variables|Default|GetMyWalkSFX)))