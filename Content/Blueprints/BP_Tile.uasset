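; BP_Tile is a tile actor that records itself as the player's current tile and displays its danger level.
; On actor overlap, it checks that the other actor is a BP_PlayerCharacter and sets that character's CurrentTile to itself.
; The construction script writes DangerLevel to a text render component, so the value is baked onto the tile when it is constructed.
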(event Collision|EventActorBeginOverlap
  (params (OtherActor :type Actor%20Object%20Reference))
  (if (Utilities|ClassIsChildOf (Utilities|GetClass OtherActor) "/Game/Character/BP_PlayerCharacter.BP_PlayerCharacter_C")
    (bind _asbp_player_character (Utilities|Casting|CastToBP_PlayerCharacter OtherActor))
    (Variables|/Game/Character/BP_PlayerCharacter.BP_PlayerCharacter_C|SetCurrentTile _asbp_player_character self)))

(event EventBeginPlay)

(event EventActorBeginOverlap
  (params (OtherActor :type Actor%20Object%20Reference)))

(event EventTick
  (params (DeltaSeconds :type Float%20%28single-precision%29)))

(fn ConstructionScript
  (Rendering|Components|TextRender|SetText (Variables|Default|GetTextRender) (Utilities|Text|ToText(Integer) (Variables|Default|GetDangerLevel))))